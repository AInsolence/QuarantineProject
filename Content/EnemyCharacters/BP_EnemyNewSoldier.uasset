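; Enemy soldier AI Blueprint that drives the Enemy blackboard key for chasing the player.
; Sensing a Player-tagged actor prints a debug string, cancels the give-up timer and stores that actor as Enemy.
; Any other perception update starts a timer that clears Enemy after a configurable chase duration.
; An OnActorOnEnemyFire dispatcher, bound at BeginPlay, sets Enemy directly to the player pawn, bypassing perception.
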(event `self.PerceptionComponent.OnTargetPerceptionUpdated`
  (params (Actor :type "Actor Object Reference") (Stimulus :type "AIStimulus Structure"))
  (if (and (`self.ActorHasTag` Actor "Player") (`.bSuccessfullySensed` (break `AIStimulus` Stimulus)))
    (`KismetSystemLibrary.PrintString` "I'm NEW SOLDIER")
    ;[1 1 1] Clear chasing timer and set values
    (`KismetSystemLibrary.K2_ClearAndInvalidateTimerHandle` (`self.EnemyTimer`))
    (`BlackboardComponent.SetValueAsObject` (`AIBlueprintHelperLibrary.GetBlackboard` (`self.GetController`)) (`self.Enemy`) Actor)
    (else
      ;[1 1 1] If AI cannot find an enemy: set timer and values in BB
      (bind _returnvalue (`KismetSystemLibrary.K2_SetTimerDelegate` (delegate `EventStartEnemyTimer`) (`self.HowLongChasingAndDoNotGiveUp`)))
      (set `self.EnemyTimer` _returnvalue))))

(event `EventStartEnemyTimer`
  ;[1 1 1] If AI cannot find an enemy: set timer and values in BB
  (`BlackboardComponent.SetValueAsObject` (`AIBlueprintHelperLibrary.GetBlackboard` (`self.GetController`)) (`self.Enemy`) null))

(event `self.ReceiveBeginPlay`
  (add `self.OnActorOnEnemyFire` (delegate `OnActorOnEnemyFire_Event_1`)))

(event `OnActorOnEnemyFire_Event_1`
  (`BlackboardComponent.SetValueAsObject` (`AIBlueprintHelperLibrary.GetBlackboard` (`self.GetController`)) (`self.Enemy`) (`GameplayStatics.GetPlayerPawn` 0)))

(fn `UserConstructionScript`)