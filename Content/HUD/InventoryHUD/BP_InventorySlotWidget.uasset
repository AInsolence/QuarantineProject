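; Inventory item widget for a grid-based HUD inventory, handling the start of drag and drop.
; When a drag is detected, it frees its slots in the owning grid, removes itself from the parent and notifies the grid of the removal.
; It then returns a drag operation carrying itself as payload and its unique ID as tag, with an enlarged, item-sized copy of the widget as the drag visual.
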(fn `OnDragDetected`
  (params (MyGeometry :type "Geometry Structure") (PointerEvent :type "PointerEvent Structure (by ref)"))
  (returns (Operation :type "DragDropOperation Object Reference"))
  (bind _currentgridowner (`self.CurrentGridOwner`))
  ;[1 1 1] Bind drag image to Drag detected event
  ;[1 1 1] Free item position in a parent container
  (bind _returnvalue (`self.GetItemSizeInInventory` self))
  (bind _returnvalue_2 (`self.GetItemPositionInInventory` self))
  (`KismetSystemLibrary.PrintString` (`KismetStringLibrary.Conv_ObjectToString` _currentgridowner))
  (`QP_InventoryUniformGridPanel.InsertItemInContainer` _currentgridowner _returnvalue _returnvalue_2 false)
  (`self.RemoveFromParent`)
  ;[1 1 1] Broadcast grid changes
  (`QP_InventoryUniformGridPanel.ItemWasRemoved` (`self.CurrentGridOwner`))
  (bind _returnvalue_3 (`|CreateWidget` (`GameplayStatics.GetObjectClass` self)))
  (`self.SetRenderScale` _returnvalue_3 (1.4 1.5))
  (bind _returnvalue_4 (`self.SetInventoryItemSize` _returnvalue_3 _returnvalue))
  (bind _returnvalue_5 (`|CreateDragDropOperation` "/Script/UMG.DragDropOperation" (`self.UniqueID`) self _returnvalue_4 "TopLeft"))
  (return _returnvalue_5))